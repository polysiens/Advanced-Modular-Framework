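; Default Game Instance that switches Game Feature plugins on or off when it initializes.
; It iterates a primary asset ID list and looks up each asset name as a row in DT_FeatureState.
; The row's Enabled flag selects a LoadGameFeaturePlugin or DeactivateGameFeaturePlugin console command built with that name.
; Each handled name is printed, as is a warning when a row is missing.
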(event `self.ReceiveInit`
  (`self.InitiateFeatures`))

(event `InitiateFeatures`
  (bind _outprimaryassetidlist (`KismetSystemLibrary.GetPrimaryAssetIdList` "GameFeatureData"))
  (for _array_element _outprimaryassetidlist
    (bind _returnvalue (`|GetDataTableRow` "/Game/DataTables/DT_FeatureState.DT_FeatureState" (`.PrimaryAssetName` (break `PrimaryAssetId` _array_element)))
      (:`then`
        (if (break `/Game/Data/FeatureState_struct` _returnvalue)
          (bind _returnvalue_2 (`KismetStringLibrary.Conv_NameToString` (`.PrimaryAssetName` (break `PrimaryAssetId` _array_element))))
          (`KismetSystemLibrary.ExecuteConsoleCommand` (`KismetStringLibrary.Concat_StrStr` "LoadGameFeaturePlugin " _returnvalue_2) null)
          (`KismetSystemLibrary.PrintString` _returnvalue_2)
          (else
            (bind _returnvalue_3 (`KismetStringLibrary.Conv_NameToString` (`.PrimaryAssetName` (break `PrimaryAssetId` _array_element))))
            (`KismetSystemLibrary.ExecuteConsoleCommand` (`KismetStringLibrary.Concat_StrStr` "DeactivateGameFeaturePlugin " _returnvalue_3) null)
            (`KismetSystemLibrary.PrintString` _returnvalue_3 true true (struct :`R` 1.0 :`G` 0.429254 :`A` 1.0)))))
      (:`RowNotFound`
        (`KismetSystemLibrary.PrintString` "Feature State Data Table Row Not Found!" true true (struct :`R` 1.0 :`A` 1.0) 5.0)))))