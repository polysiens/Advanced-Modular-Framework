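; Core Game Instance that bootstraps feature plugin loading when the game starts.
; On Init it constructs and stores a FeatureManager object, then hands it the InitPlugins variable to begin loading.
; It then queries the Asset Manager for Progression01 primary assets and prints their names and count as debug output.
; A SpawnActor helper wraps actor spawning with a given class, transform and collision handling.
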(event `self.ReceiveInit`
  (`self.FeaturePluginManagerSetup`)
  (bind _outprimaryassetidlist (`KismetSystemLibrary.GetPrimaryAssetIdList` (make `PrimaryAssetType` "Progression01")))
  (for _array_element _outprimaryassetidlist
    (`KismetSystemLibrary.PrintString` (`KismetStringLibrary.Conv_NameToString` (`.PrimaryAssetName` (break `PrimaryAssetId` _array_element)))))
  (`KismetSystemLibrary.PrintString` (`KismetStringLibrary.Conv_IntToString` (`KismetArrayLibrary.Array_Length` _outprimaryassetidlist))))

(fn `FeaturePluginManagerSetup`
  (bind _returnvalue (`|GenericCreateObject` "/Game/FeatureManager/Blueprints/FeatureManager.FeatureManager_C"))
  (set `self.FeatureManager` _returnvalue)
  (`/Game/FeatureManager/Blueprints/FeatureManager.InitFeaturePluginLoad` _returnvalue (`self.InitPlugins`)))

(fn `SpawnActor`
  (params (Class :type "Actor Class Reference") (SpawnTransform :type "Transform Structure") (CollisionHandlingOverride :type "ESpawnActorCollisionHandlingMethod Enum" :default "Undefined"))
  (returns (ReturnValue :type "Actor Object Reference"))
  (bind _returnvalue (`|SpawnActorFromClass` Class SpawnTransform CollisionHandlingOverride "MultiplyWithRoot" null null))
  (return _returnvalue))