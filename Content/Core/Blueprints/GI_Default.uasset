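; Default Game Instance Blueprint that bootstraps feature plugin loading when the game instance initializes.
; On Init it constructs and stores a FeatureManager object, then passes it the InitPlugins variable to start loading.
; It then queries the Asset Manager for Progression01 primary assets and prints each asset name and the total count, apparently as a debug check.
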(event `self.ReceiveInit`
  (`self.FeaturePluginManagerSetup`)
  (bind _outprimaryassetidlist (`KismetSystemLibrary.GetPrimaryAssetIdList` (make `PrimaryAssetType` "Progression01")))
  (for _array_element _outprimaryassetidlist
    (`KismetSystemLibrary.PrintString` (`KismetStringLibrary.Conv_NameToString` (`.PrimaryAssetName` (break `PrimaryAssetId` _array_element)))))
  (`KismetSystemLibrary.PrintString` (`KismetStringLibrary.Conv_IntToString` (`KismetArrayLibrary.Array_Length` _outprimaryassetidlist))))

(fn `FeaturePluginManagerSetup`
  (bind _returnvalue (`|GenericCreateObject` "/Game/FeatureManager/Blueprints/FeatureManager.FeatureManager_C"))
  (set `self.FeatureManager` _returnvalue)
  (`/Game/FeatureManager/Blueprints/FeatureManager.InitFeaturePluginLoad` _returnvalue (`self.InitPlugins`)))