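; Feature manager that loads and unloads Game Feature plugins through console commands, driven by rows in DT_FeatureState.
; FeatureSetup records enabled rows with their dependencies, pools disallowed names, and unloads disabled rows while keeping them registered.
; It prints dependency conflicts, then unloads disallowed features and loads the rest.
; The dependency-loading branch checks the parent against Enabled after adding it, so dependencies never load there.
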(event `InitFeatureLoad`
  (`self.FeatureSetup`))

(fn `FeatureSetup`
  (locals (TempFeatureName :type Name) (Disallowed :type "Array of Name") (Enabled :type "Array of Name") (CurrentIndex :type Integer))
  (bind _features (`self.Features`))
  (bind _outrownames (`DataTableFunctionLibrary.GetDataTableRowNames` "/Game/FeatureManager/DataTables/DT_FeatureState.DT_FeatureState"))
  (for _array_element _outrownames
    (set `local.TempFeatureName` _array_element)
    (bind _returnvalue (`|GetDataTableRow` "/Game/FeatureManager/DataTables/DT_FeatureState.DT_FeatureState" _array_element)
      (:`then`
        (if (break `/Game/FeatureManager/Data/FeatureState_struct` _returnvalue)
          (`BlueprintMapLibrary.Map_Add` (`self.Features`) (`local.TempFeatureName`) (make `/Game/FeatureManager/Data/DependencyArray_struct` (`.Dependencies_11_F0C7EC904939EE66D80B009C757BC38F` (break `/Game/FeatureManager/Data/FeatureState_struct` _returnvalue)) (`.Disallowed_13_C8B7DFBF4DDA96C8F8FE77A53E0D62E0` (break `/Game/FeatureManager/Data/FeatureState_struct` _returnvalue))))
          (for _array_element_2 (`.Disallowed_13_C8B7DFBF4DDA96C8F8FE77A53E0D62E0` (break `/Game/FeatureManager/Data/FeatureState_struct` _returnvalue))
            (`KismetArrayLibrary.Array_AddUnique` (`local.Disallowed`) _array_element_2))
          (else
            (`self.UnloadAndKeepRegisteredFeature` (`local.TempFeatureName`)))))))
  (`|ExecutionSequence`
    (:`then_0`
      (bind _keys (`BlueprintMapLibrary.Map_Keys` _features))
      (bind _values (`BlueprintMapLibrary.Map_Values` _features))
      (for (_array_element_3 _array_index) _values
        (for _array_element_4 (break `/Game/FeatureManager/Data/DependencyArray_struct` _array_element_3)
          (if (`KismetArrayLibrary.Array_Contains` (`local.Disallowed`) _array_element_4)
            (`KismetSystemLibrary.PrintString` null (`KismetStringLibrary.Concat_StrStr` "DEPENDENCY CONFLICT FOUND IN: " (`KismetStringLibrary.Conv_NameToString` (`|GetArrayItem` _keys _array_index))) true true (struct :`R` 1.0 :`A` 1.0))))))
    (:`then_1`
      (bind _keys_2 (`BlueprintMapLibrary.Map_Keys` (`self.Features`)))
      (for (_array_element_5 _array_index_2) _keys_2
        (set `local.TempFeatureName` _array_element_5)
        (set `local.CurrentIndex` _array_index_2)
        (if (`KismetArrayLibrary.Array_Contains` (`local.Disallowed`) (`local.TempFeatureName`))
          (`self.UnloadAndKeepRegisteredFeature` (`local.TempFeatureName`))
          (else
            (bind _returnvalue_2 (`|GetDataTableRow` "/Game/FeatureManager/DataTables/DT_FeatureState.DT_FeatureState" (`local.TempFeatureName`))
              (:`then`
                (if (and (break `/Game/FeatureManager/Data/FeatureState_struct` _returnvalue_2) (not (`KismetArrayLibrary.Array_Contains` (`local.Enabled`) (`local.TempFeatureName`))))
                  (`|ExecutionSequence`
                    (:`then_0`
                      (`self.LoadFeature` (`local.TempFeatureName`))
                      (`KismetArrayLibrary.Array_Add` (`local.Enabled`) (`local.TempFeatureName`)))
                    (:`then_1`
                      (for _array_element_6 (`.Dependencies_11_F0C7EC904939EE66D80B009C757BC38F` (break `/Game/FeatureManager/Data/FeatureState_struct` _returnvalue_2))
                        (if (and (not (`KismetArrayLibrary.Array_Contains` (`local.Disallowed`) _array_element_6)) (not (`KismetArrayLibrary.Array_Contains` (`local.Enabled`) (`local.TempFeatureName`))))
                          (`self.LoadFeature` _array_element_6)
                          (`KismetArrayLibrary.Array_Add` (`local.Enabled`) _array_element_6))))))))))))))

(fn `LoadFeature`
  (params (FeatureName :type Name))
  (bind _returnvalue (`KismetStringLibrary.Conv_NameToString` FeatureName))
  (`KismetSystemLibrary.ExecuteConsoleCommand` null (`KismetStringLibrary.Concat_StrStr` "LoadGameFeaturePlugin " _returnvalue) null)
  (`KismetSystemLibrary.PrintString` null _returnvalue))

(fn `UnloadAndKeepRegisteredFeature`
  (params (FeatureName :type Name))
  (bind _returnvalue (`KismetStringLibrary.Conv_NameToString` FeatureName))
  (`KismetSystemLibrary.ExecuteConsoleCommand` null (`KismetStringLibrary.Concat_StrStr` "UnloadAndKeepRegisteredGameFeaturePlugin " _returnvalue) null)
  (`KismetSystemLibrary.PrintString` null _returnvalue true true (struct :`R` 1.0 :`G` 0.429254 :`A` 1.0)))